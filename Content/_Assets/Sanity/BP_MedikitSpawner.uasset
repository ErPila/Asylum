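; BP_MedikitSpawner is a respawning health pickup that heals characters on contact.
; When a BP_BaseCharacter below max HP overlaps the sphere while the kit is available, it adds Health to the Combat component's HP, capped at max.
; It then hides the Medikit and starts a timer that restores availability and visibility after TimeSpawn.
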(event OnComponentBeginOverlap(Sphere)
  (params (OverlappedComponent :type Primitive%20Component%20Object%20Reference) (OtherActor :type Actor%20Object%20Reference) (OtherComp :type Primitive%20Component%20Object%20Reference) (OtherBodyIndex :type Integer) (bFromSweep :type Boolean) (SweepResult :type Hit%20Result%20Structure%20%28by%20ref%29))
  (if (Variables|Default|GetCanTake?)
    (bind _asbp_base_character (Utilities|Casting|CastToBP_BaseCharacter OtherActor))
    (if (< (Class|Combat|GetActualHp (Class|BaseChar|GetCombat _asbp_base_character)) (Class|Combat|GetMaxHp (Class|BaseChar|GetCombat _asbp_base_character)))
      (if (> (+ (Class|Combat|GetActualHp (Class|BaseChar|GetCombat _asbp_base_character)) (Variables|Default|GetHealth)) (Class|Combat|GetMaxHp (Class|BaseChar|GetCombat _asbp_base_character)))
        (Class|Combat|SetActualHp (Class|BaseChar|GetCombat _asbp_base_character) (Class|Combat|GetMaxHp (Class|BaseChar|GetCombat _asbp_base_character)))
        (else
          (Class|Combat|SetActualHp (Class|BaseChar|GetCombat _asbp_base_character) (+ (Class|Combat|GetActualHp (Class|BaseChar|GetCombat _asbp_base_character)) (Variables|Default|GetHealth)))))
      (bind _output_get (Variables|Default|SetCanTake? false))
      (Rendering|SetVisibility (Variables|Default|GetMedikit) _output_get false)
      (Utilities|Time|SetTimerbyEvent (delegate Custom|ResetState) (Variables|Default|GetTimeSpawn)))))

(event Custom|ResetState
  (bind _output_get (Variables|Default|SetCanTake? true))
  (Rendering|SetVisibility (Variables|Default|GetMedikit) _output_get false))

(event EventBeginPlay)

(event Collision|EventActorBeginOverlap
  (params (OtherActor :type Actor%20Object%20Reference)))

(event EventTick
  (params (DeltaSeconds :type Float%20%28single-precision%29)))

(fn ConstructionScript)