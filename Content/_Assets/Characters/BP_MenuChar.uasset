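; BP_MenuChar is a menu display actor that shows a character model with a looping idle animation.
; On BeginPlay, if GetSelected is set, it reads SelectedCharacter from the AsylumInstance game instance.
; That value picks one of three skeletal meshes (Ange, Chri or Luca), each playing the same Idle_Large animation.
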(event EventBeginPlay
  (bind _skeletalmesh (Variables|Default|GetSkeletalMesh))
  (if (Variables|Default|GetGetSelected?)
    (bind _asasylum_instance (Utilities|Casting|CastToAsylumInstance (Game|GetGameInstance)))
    (switch int (Math|Conversions|ToInteger(Byte) (Variables|/Script/Asylum.AsylumInstance|GetSelectedCharacter _asasylum_instance))
      (:0
        (Components|SkeletalMesh|SetSkeletalMeshAsset _skeletalmesh "/Game/_Assets/Characters/Angelica/Ange_Mesh.Ange_Mesh")
        (Components|Animation|PlayAnimation (Variables|Default|GetSkeletalMesh) "/Game/_Assets/Animations/AnimationAnge/Idle_Large.Idle_Large" true))
      (:1
        (Components|SkeletalMesh|SetSkeletalMeshAsset _skeletalmesh "/Game/_Assets/Characters/Christian/Chri_Mesh.Chri_Mesh")
        (Components|Animation|PlayAnimation (Variables|Default|GetSkeletalMesh) "/Game/_Assets/Animations/AnimationChristian/Idle_Large.Idle_Large" true))
      (:2
        (Components|SkeletalMesh|SetSkeletalMeshAsset _skeletalmesh "/Game/_Assets/Characters/Luca/Luca_Mesh.Luca_Mesh")
        (Components|Animation|PlayAnimation (Variables|Default|GetSkeletalMesh) "/Game/_Assets/Animations/AnimationLuca/Idle_Large.Idle_Large" true)))))

(event Collision|EventActorBeginOverlap
  (params (OtherActor :type Actor%20Object%20Reference)))

(event EventTick
  (params (DeltaSeconds :type Float%20%28single-precision%29)))

(fn ConstructionScript)