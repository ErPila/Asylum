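; Base character Blueprint that provides a torch, local stats HUD, win/lose widget and pause menu.
; BeginPlay creates the widgets and a dynamic torch material.
; Torch toggling chains through Server and Multicast events to set spotlight intensity and emissive from TorchOn, while SetChange applies mesh and offsets locally or via a similar chain when not locally controlled.
; IA_Pause flip-flops the menu, switching input mode and cursor.
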(event Custom|Multicast
  (bind _spotlight (Variables|Default|GetSpotLight))
  (if (Variables|Default|GetbTorchOn)
    (Rendering|Components|Light|SetIntensity _spotlight (Variables|Default|GetIntensity%20Light))
    (Rendering|Material|SetScalarParameterValue (Variables|Default|GetTorch%20Material) "Emissive" 0.1 :!class /Script/Engine.MaterialInstanceDynamic)
    (else
      (Rendering|Components|Light|SetIntensity _spotlight 0.0)
      (Rendering|Material|SetScalarParameterValue (Variables|Default|GetTorch%20Material) "Emissive" 0.0 :!class /Script/Engine.MaterialInstanceDynamic))))

(event Custom|Server
  (CallFunction|Multicast))

(event Custom|OpenPauseMenu
  (bind _returnvalue (Game|GetPlayerController 0))
  (Variables|Default|GetPauseMenu
    (:then
      _)
    (:else
      (bind _returnvalue_2 (UserInterface|CreateWidget "/Game/_Assets/UI/WBP_Pause.WBP_Pause_C" (Game|GetPlayerController 0)))
      (bind _output_get (Variables|Default|SetPauseMenu _returnvalue_2))
      (Variables|/Game/_Assets/UI/WBP_Pause.WBP_Pause_C|SetPlayer _output_get self)))
  (UserInterface|Viewport|AddtoViewport (Variables|Default|GetPauseMenu) 0)
  (Input|DisableInput _returnvalue)
  (Variables|/Script/Engine.PlayerController|SetbShowMouseCursor _returnvalue true)
  (Input|SetInputModeUIOnly _returnvalue 0 "DoNotLock" false))

(event Custom|ClosePauseMenu
  (bind _returnvalue (Game|GetPlayerController 0))
  (Widget|RemovefromParent (Variables|Default|GetPauseMenu))
  (Input|EnableInput _returnvalue)
  (Variables|/Script/Engine.PlayerController|SetbShowMouseCursor _returnvalue false)
  (Input|SetInputModeGameOnly _returnvalue false))

(event Custom|ServerSetTorcia
  (CallFunction|MulticastSetTorcia))

(event Custom|MulticastSetTorcia
  (Components|StaticMesh|SetStaticMesh (Variables|Default|GetTorciaComponent) (Variables|Default|GetTorcia))
  (Transformation|SetRelativeTransform (Variables|Default|GetTorciaComponent) (Math|Transform|MakeTransform (Variables|Default|GetTorciaLocationOffset) (Variables|Default|GetTorciaRotationOffset) (Variables|Default|GetTorciaScaleOffset)) false false)
  (Transformation|SetRelativeTransform (Variables|Default|GetSpotLight) (Math|Transform|MakeTransform (Variables|Default|GetLuceLocationOffset) (Variables|Default|GetLuceRotationOffset) "1.000000,1.000000,1.000000") false false))

(event Input|EnhancedActionEvents|EnhancedInputActionIA_Pause
  (params (ActionValue :type Boolean) (ElapsedSeconds :type Float%20%28double-precision%29) (TriggeredSeconds :type Float%20%28double-precision%29) (InputAction :type Input%20Action%20Object%20Reference :default "/Game/_Assets/Inputs/IA_Pause.IA_Pause"))
  (:Started
    (Utilities|FlowControl|FlipFlop
      (:A
        (CallFunction|OpenPauseMenu))
      (:B
        (CallFunction|ClosePauseMenu)))))

(event EventBeginPlay
  (if (Pawn|IsLocallyControlled)
    (bind _returnvalue (UserInterface|CreateWidget "/Game/_Assets/UI/WBP_PStats.WBP_PStats_C" 0 self))
    (Variables|Default|SetHUD _returnvalue)
    (UserInterface|Viewport|AddtoViewport _returnvalue 0))
  (bind _returnvalue_2 (Rendering|Material|CreateDynamicMaterialInstance (Variables|Default|GetTorciaComponent) 0 "/Game/_Assets/Materials/MI_Light.MI_Light" "None" :!class /Script/Engine.PrimitiveComponent))
  (bind _output_get (Variables|Default|SetTorch%20Material _returnvalue_2))
  (Rendering|Material|SetScalarParameterValue _output_get "Emissive" 0.0 :!class /Script/Engine.MaterialInstanceDynamic)
  (bind _returnvalue_3 (UserInterface|CreateWidget "/Game/_Assets/UI/WBP_LoseWin.WBP_LoseWin_C" 0 self))
  (Variables|Default|SetEndGameWidget _returnvalue_3))

(event Collision|EventActorBeginOverlap
  (params (OtherActor :type Actor%20Object%20Reference)))

(event EventTick
  (params (DeltaSeconds :type Float%20%28single-precision%29)))

(event EventAttivaDisattivaTorcia
  (CallFunction|Server))

(event EventSetChange
  (if (Pawn|IsLocallyControlled)
    (Components|StaticMesh|SetStaticMesh (Variables|Default|GetTorciaComponent) (Variables|Default|GetTorcia))
    (Transformation|SetRelativeTransform (Variables|Default|GetTorciaComponent) (Math|Transform|MakeTransform (Variables|Default|GetTorciaLocationOffset) (Variables|Default|GetTorciaRotationOffset) (Variables|Default|GetTorciaScaleOffset)) false false)
    (Transformation|SetRelativeTransform (Variables|Default|GetSpotLight) (Math|Transform|MakeTransform (Variables|Default|GetLuceLocationOffset) (Variables|Default|GetLuceRotationOffset) "1.000000,1.000000,1.000000") false false)
    (else
      (CallFunction|ServerSetTorcia))))

(fn ConstructionScript)