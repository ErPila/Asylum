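; BP_Luce is an environment light fixture with a wall or ceiling variant, an on/off state and optional flicker.
; The Construction Script uses Tipo to pick the mesh and either a point or rect light, creates a dynamic emissive material, and applies the TurnOn state.
; When Flicker and TurnOn are set, BeginPlay starts a randomly timed, self-rescheduling timer that toggles light intensity and emissive together.
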(event Custom|FlickerEvent
  (if (== (Variables|/Script/Engine.LightComponentBase|GetIntensity (Variables|Default|GetLight)) 0.0)
    (Rendering|Components|Light|SetIntensity (Variables|Default|GetLight) (Variables|Default|GetIntensity))
    (Rendering|Material|SetScalarParameterValue (Variables|Default|GetMaterial) "Emissive" 0.1 :!class /Script/Engine.MaterialInstanceDynamic)
    (else
      (Rendering|Components|Light|SetIntensity (Variables|Default|GetLight) 0.0)
      (Rendering|Material|SetScalarParameterValue (Variables|Default|GetMaterial) "Emissive" 0.0 :!class /Script/Engine.MaterialInstanceDynamic)))
  (Utilities|Time|SetTimerbyEvent (delegate Custom|FlickerEvent) (Math|Random|RandomFloatinRange (Variables|Default|GetMinFlickerTime) (Variables|Default|GetMaxFlickerTime))))

(event EventBeginPlay
  (if (and (Variables|Default|GetFlicker?) (Variables|Default|GetTurnOn))
    (Utilities|Time|SetTimerbyEvent (delegate Custom|FlickerEvent) (Math|Random|RandomFloatinRange (Variables|Default|GetMinFlickerTime) (Variables|Default|GetMaxFlickerTime)))))

(event EventTick
  (params (DeltaSeconds :type Float%20%28single-precision%29)))

(fn ConstructionScript
  (Utilities|FlowControl|Sequence
    (:then_0
      (switch int (Variables|Default|GetTipo)
        (:0
          (Components|StaticMesh|SetStaticMesh (Variables|Default|GetLuce) "/Game/_Assets/Gfx/Environment/Luce_Muro/Luce_Muro.Luce_Muro")
          (Variables|Default|SetLight (Variables|Default|GetPointLight))
          (bind _returnvalue (Rendering|Material|CreateDynamicMaterialInstance (Variables|Default|GetLuce) 0 "/Game/_Assets/Materials/MI_Light.MI_Light" "None" :!class /Script/Engine.PrimitiveComponent))
          (Variables|Default|SetMaterial _returnvalue))
        (:1
          (Components|StaticMesh|SetStaticMesh (Variables|Default|GetLuce) "/Game/_Assets/Gfx/Environment/Luce_Soffitto/Luce_Soffitto_2_Luce_Soffitto.Luce_Soffitto_2_Luce_Soffitto")
          (Variables|Default|SetLight (Variables|Default|GetRectLight))
          (bind _returnvalue_2 (Rendering|Material|CreateDynamicMaterialInstance (Variables|Default|GetLuce) 1 "/Game/_Assets/Materials/MI_Light.MI_Light" "None" :!class /Script/Engine.PrimitiveComponent))
          (Variables|Default|SetMaterial _returnvalue_2))))
    (:then_1
      (if (Variables|Default|GetTurnOn)
        (Rendering|Components|Light|SetIntensity (Variables|Default|GetLight) (Variables|Default|GetIntensity))
        (Rendering|Material|SetScalarParameterValue (Variables|Default|GetMaterial) "Emissive" 0.1 :!class /Script/Engine.MaterialInstanceDynamic)
        (else
          (Rendering|Components|Light|SetIntensity (Variables|Default|GetLight) 0.0)
          (Rendering|Material|SetScalarParameterValue (Variables|Default|GetMaterial) "Emissive" 0.0 :!class /Script/Engine.MaterialInstanceDynamic))))))