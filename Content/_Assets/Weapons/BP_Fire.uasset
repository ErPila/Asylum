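; BP_Fire is a fire area actor that damages characters standing in it and destroys itself after ten seconds.
; A BaseChar entering or leaving its sphere opens or closes a single gate on Tick.
; While open, the gate applies Danni scaled by delta time to the combat component of the last character to enter, and writes that amount to its Damage variable.
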(event OnComponentBeginOverlap(Sphere)
  (params (OverlappedComponent :type Primitive%20Component%20Object%20Reference) (OtherActor :type Actor%20Object%20Reference) (OtherComp :type Primitive%20Component%20Object%20Reference) (OtherBodyIndex :type Integer) (bFromSweep :type Boolean) (SweepResult :type Hit%20Result%20Structure%20%28by%20ref%29))
  (bind _asbase_char (Utilities|Casting|CastToBaseChar OtherActor))
  (CallFunction|StartDamage _asbase_char))

(event OnComponentEndOverlap(Sphere)
  (params (OverlappedComponent :type Primitive%20Component%20Object%20Reference) (OtherActor :type Actor%20Object%20Reference) (OtherComp :type Primitive%20Component%20Object%20Reference) (OtherBodyIndex :type Integer))
  (Utilities|Casting|CastToBaseChar OtherActor)
  (CallFunction|EndDamage))

(event Custom|EndDamage
  (bind _danni (Variables|Default|GetDanni))
  (Utilities|FlowControl|Gate true) ; enters at Close
)

(event Custom|StartDamage
  (params (Player :type Base%20Char%20Object%20Reference))
  (bind _danni (Variables|Default|GetDanni))
  (Utilities|FlowControl|Gate true) ; enters at Open
)

(event EventBeginPlay
  (Utilities|FlowControl|Delay 1e+01)
  (Actor|DestroyActor))

(event EventTick
  (params (DeltaSeconds :type Float%20%28single-precision%29))
  (bind _danni (Variables|Default|GetDanni))
  (Utilities|FlowControl|Gate true
    (:Exit
      (Class|Combat|ReceiveDamage (Class|BaseChar|GetCombat (stale Custom|StartDamage Player)) (* _danni DeltaSeconds))
      (Variables|/Script/Asylum.BaseChar|SetDamage (stale Custom|StartDamage Player) (* _danni DeltaSeconds)))))

(fn ConstructionScript)